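; World actor that displays an Easy Input Prompts multi-key prompt through a widget component, using the configured display space.
; On BeginPlay it creates the multi-prompt displayer widget from the key definitions, styling and spacing, then assigns it to the component.
; For adjustable sharpness, it multiplies icon and font sizes by a resolution multiplier and divides the component's world scale by the same factor.
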(event `self.ReceiveBeginPlay`
  (bind _resolutionmultiplier (`self.ResolutionMultiplier`))
  (bind _widget (`self.Widget`))
  (bind (_iconsize _additionaltext _textstyling _textcolor _textposition _textpadding _iconcolor _overlaymaterial _overlaymaterialtextureparametername) (break `/Game/EasyInputPrompts/Datas/F_InputPromptStyling` (`self.StylingDefinition`)))
  (bind ((`Font_10_52B1FFAB4D33127D79DF0FA04DF32F8B` _font)) (break `/Game/EasyInputPrompts/Datas/F_CommonTextInfo` _textstyling))
  (bind _structout (setmembers `SlateFontInfo` :`StructRef` _font :`Size` (* (`.Size` (break `SlateFontInfo` _font)) _resolutionmultiplier)))
  (bind _structout_2 (setmembers `/Game/EasyInputPrompts/Datas/F_CommonTextInfo` :`StructRef` _textstyling :`Font` _structout))
  (bind _returnvalue (`|CreateWidget` "/Game/EasyInputPrompts/Core/WBP_EasyMultiInputPromptDisplayer.WBP_EasyMultiInputPromptDisplayer_C" null (`self.KeysDefinition`) (make `/Game/EasyInputPrompts/Datas/F_InputPromptStyling` (* _iconsize _resolutionmultiplier) _additionaltext _structout_2 _textcolor _textposition _textpadding _iconcolor _overlaymaterial _overlaymaterialtextureparametername) (`self.Spacing`)))
  (bind _output_get (set `self.MutliInputPromptWidgetReference` _returnvalue))
  (`WidgetComponent.SetWidget` (`self.Widget`) _output_get)
  (`SceneComponent.SetWorldScale3D` _widget (/ (`SceneComponent.K2_GetComponentScale` _widget) (`self.ResolutionMultiplier`))))

(fn `UserConstructionScript`
  (`WidgetComponent.SetWidgetSpace` (`self.Widget`) (`self.DisplayType`)))