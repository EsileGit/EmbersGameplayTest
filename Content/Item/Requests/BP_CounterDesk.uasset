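; Counter desk actor where requests are drafted, cancelled and fulfilled with parcels, presenting the state of the active request.
; BeginPlay binds two child-actor buttons to drafting and cancelling, and hands itself to the request widget.
; Request events, apparently from the parent class, toggle button interactivity and customer visibility and play 2D sounds.
; The spotlight color shows active or success, and briefly flashes wrong when a parcel is rejected.
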(event `self.ReceiveBeginPlay`
  (`|ExecutionSequence`
    (:`then_0`
      ; Init buttons
      (bind _asbp_interaction_button (cast `/Game/LevelPrototyping/Blueprint/BP_InteractionButton` (`ChildActorComponent.ChildActor` (`self.Button_Request`))))
      (bind _output_get (set `self.InteractionButton_Request` _asbp_interaction_button))
      (add `/Game/LevelPrototyping/Blueprint/BP_InteractionButton.OnButtonHasBeenInteracted` _output_get (`|CreateDelegate` :!event `Button_TryDraftNewRequest`))
      (bind _asbp_interaction_button_2 (cast `/Game/LevelPrototyping/Blueprint/BP_InteractionButton` (`ChildActorComponent.ChildActor` (`self.Button_Cancel`))))
      (bind _output_get_2 (set `self.InteractionButton_Cancel` _asbp_interaction_button_2))
      (add `/Game/LevelPrototyping/Blueprint/BP_InteractionButton.OnButtonHasBeenInteracted` _output_get_2 (`|CreateDelegate` :!event `Button_CancelCurrentRequest`)))
    (:`then_1`
      (`/Game/LevelPrototyping/Blueprint/BP_InteractionButton.SetCanBeInteracted` (`self.InteractionButton_Request`) true)
      (`/Game/LevelPrototyping/Blueprint/BP_InteractionButton.SetCanBeInteracted` (`self.InteractionButton_Cancel`) false))
    (:`then_2`
      ; Init UI
      (bind _asegt_counter_desk_widget (cast `EGT_CounterDeskWidget` (`WidgetComponent.GetWidget` (`self.Widget_Request`))))
      (`EGT_CounterDeskWidget.SetCounterDesk` _asegt_counter_desk_widget self)
      (`SceneComponent.SetVisibility` (`self.Customer`) false true))))

(event `self.OnNoRequestAvailable`
  (`GameplayStatics.PlaySound2D` "/Game/SFX/Interaction/error_007.error_007" 1.0 1.0 0.0 null null)
  (`/Game/LevelPrototyping/Blueprint/BP_InteractionButton.SetCanBeInteracted` (`self.InteractionButton_Request`) false)
  (`SceneComponent.SetVisibility` (`self.Customer`) false true))

(event `Button_CancelCurrentRequest`
  ; Button actions
  (`self.CancelActiveRequest`))

(event `self.OnParcelRejected`
  (params (Parcel :type "EGT_ParcelBase Object Reference") (Request :type "EGT_Request Structure (by ref)"))
  (`GameplayStatics.PlaySound2D` "/Game/SFX/Interaction/error_005.error_005" 1.0 1.0 0.0 null null)
  ; Blink wrong
  (`LightComponent.SetLightColor` (`self.SpotLight`) (`self.LightColor_Wrong`) true)
  (`KismetSystemLibrary.Delay` 0.8) ; This shouldn't cause the light to show if hidden during delay (it just changes the color)
  (`LightComponent.SetLightColor` (`self.SpotLight`) (`self.LightColor_Active`) true))

(event `Button_TryDraftNewRequest`
  ; Button actions
  (`self.TryDraftRequest`))

(event `self.OnRequestCancelled`
  (params (Request :type "EGT_Request Structure (by ref)"))
  (`GameplayStatics.PlaySound2D` "/Game/SFX/Interaction/error_007.error_007" 1.0 1.0 0.0 null null)
  (`/Game/LevelPrototyping/Blueprint/BP_InteractionButton.SetCanBeInteracted` (`self.InteractionButton_Cancel`) false)
  (`SceneComponent.SetVisibility` (`self.Customer`) false true))

(event `self.OnRequestFulfilled`
  (params (Parcel :type "EGT_ParcelBase Object Reference") (Request :type "EGT_Request Structure (by ref)") (Points :type Integer))
  (`GameplayStatics.PlaySound2D` "/Game/SFX/Interaction/confirmation_001.confirmation_001" 1.0 1.0 0.0 null null)
  (`LightComponent.SetLightColor` (`self.SpotLight`) (`self.LightColor_Success`) true)
  (`KismetSystemLibrary.Delay` 1.0)
  (`SceneComponent.SetVisibility` (`self.Customer`) false true))

(event `self.OnRequestDrafted`
  (params (Request :type "EGT_Request Structure (by ref)"))
  (`/Game/LevelPrototyping/Blueprint/BP_InteractionButton.SetCanBeInteracted` (`self.InteractionButton_Cancel`) true)
  (`LightComponent.SetLightColor` (`self.SpotLight`) (`self.LightColor_Active`) true)
  (`SceneComponent.SetVisibility` (`self.Customer`) true true))

(fn `UserConstructionScript`)