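; BP_ParcelBase is the base parcel item, adding sound feedback to focus, grab and impact events.
; Focus extends the parent behavior with a quiet 2D rollover sound; grabbing plays a 2D grab sound, both with slight random pitch variation.
; Impacts play a sound at the parcel's location, with volume following impact intensity, clamped so weak hits stay audible.
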(event `self.OnFocusBegin`
  (params (Interactor :type "Actor Object Reference"))
  (`parent.OnFocusBegin` Interactor)
  (`GameplayStatics.PlaySound2D` "/Game/SFX/Interaction/rollover3.rollover3" 0.03 (`KismetMathLibrary.RandomFloatInRange` 0.95 1.05) 0.0 null null) ; Actually not sure it's not just too much
)

(event `self.OnParcelGrabbed`
  (params (Carrier :type "Actor Object Reference"))
  (`GameplayStatics.PlaySound2D` (`self.GrabSound`) 0.2 (`KismetMathLibrary.RandomFloatInRange` 0.95 1.05) 0.0 null null) ; TODO: make it depend of parcel type
)

(event `self.OnParcelImpact`
  (params (ImpactSpeed :type "Float (single-precision)") (ImpactIntensity :type "Float (single-precision)") (Hit :type "HitResult Structure (by ref)"))
  (`GameplayStatics.PlaySoundAtLocation` (`self.ImpactSound`) (`self.K2_GetActorLocation`) (struct) (`KismetMathLibrary.FClamp` ImpactIntensity 0.15) 1.0 0.0 null null null null))

(fn `UserConstructionScript`)