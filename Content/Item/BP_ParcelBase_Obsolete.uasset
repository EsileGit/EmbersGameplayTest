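; Obsolete base Blueprint for a parcel item that changes its look when focused.
; Focus begin and end events swap the first material slot of ItemMesh between Xray and SandMesh.
; The construction script creates a dynamic instance of that slot's material and stores it in MeshMI, which the focus events do not use.
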(event `self.OnFocusBegin`
  (params (Interactor :type "Actor Object Reference"))
  (`PrimitiveComponent.SetMaterial` (`self.ItemMesh`) 0 "/Engine/VREditor/TransformGizmo/Xray.Xray"))

(event `self.OnFocusEnd`
  (params (Interactor :type "Actor Object Reference"))
  (`PrimitiveComponent.SetMaterial` (`self.ItemMesh`) 0 "/Landmass/Landscape/OldPrototype_BP/Mats/Preview/SandMesh.SandMesh"))

(fn `UserConstructionScript`
  (bind _returnvalue (`PrimitiveComponent.CreateDynamicMaterialInstance` (`self.ItemMesh`) 0 (`PrimitiveComponent.GetMaterial` (`self.ItemMesh`) 0) "None"))
  (set `self.MeshMI` _returnvalue))